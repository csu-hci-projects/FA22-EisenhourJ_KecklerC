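; BP_LightSquare is a toggleable puzzle tile that switches its mesh between a plain and a blue lit material.
; Hit calls LightSquare, which flips the tile's state and passes its SquareIndex to LightOthers on the LightSquareGameStorage game instance.
; AreaLight performs the same toggle without that notification, so it does not propagate further.
; BeginPlay prints the tile's index.
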(event `AreaLight`
  (if (`self.IsLit`)
    (`PrimitiveComponent.SetMaterial` (`self.StaticMeshComponent`) 0 "/Game/LevelPrototyping/Materials/M_Solid.M_Solid")
    (set `self.IsLit` false)
    (else
      (`PrimitiveComponent.SetMaterial` (`self.StaticMeshComponent`) 0 "/Game/LevelPrototyping/Materials/MI_Solid_Blue.MI_Solid_Blue")
      (set `self.IsLit` true))))

(event `LightSquare`
  (if (`self.IsLit`)
    (`PrimitiveComponent.SetMaterial` (`self.StaticMeshComponent`) 0 "/Game/LevelPrototyping/Materials/M_Solid.M_Solid")
    (set `self.IsLit` false)
    (bind _aslight_square_game_storage (cast `/Game/LightSquareGameStorage` (`GameplayStatics.GetGameInstance`)))
    (`/Game/LightSquareGameStorage.LightOthers` _aslight_square_game_storage (`self.SquareIndex`))
    (else
      (`PrimitiveComponent.SetMaterial` (`self.StaticMeshComponent`) 0 "/Game/LevelPrototyping/Materials/MI_Solid_Blue.MI_Solid_Blue")
      (set `self.IsLit` true)
      (bind _aslight_square_game_storage_2 (cast `/Game/LightSquareGameStorage` (`GameplayStatics.GetGameInstance`)))
      (`/Game/LightSquareGameStorage.LightOthers` _aslight_square_game_storage_2 (`self.SquareIndex`)))))

(event `self.ReceiveHit`
  (params (MyComp :type "PrimitiveComponent Object Reference") (Other :type "Actor Object Reference") (OtherComp :type "PrimitiveComponent Object Reference") (bSelfMoved :type Boolean) (HitLocation :type "Vector Structure") (HitNormal :type "Vector Structure") (NormalImpulse :type "Vector Structure") (Hit :type "HitResult Structure (by ref)"))
  (`self.LightSquare`))

(event `self.ReceiveBeginPlay`
  (`KismetSystemLibrary.PrintString` (`KismetStringLibrary.Conv_IntToString` (`self.SquareIndex`))))

(fn `UserConstructionScript`)